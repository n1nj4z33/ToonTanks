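; Game mode Blueprint for Toon Tanks that shows the start and end screens of a match.
; StartGame creates the start-game widget and adds it to the viewport.
; GameOver shows the end-game widget with win or lose text chosen by its WonGame flag, then reveals the mouse cursor and pauses the game.
; The graph only defines these event responses and contains no logic that decides when a match starts or ends.
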(event `self.StartGame`
  (bind _returnvalue (`|CreateWidget` "/Game/Blueprints/Widgets/WBP_StartGameWidget.WBP_StartGameWidget_C"))
  (`UserWidget.AddToViewport` _returnvalue 0))

(event `self.GameOver`
  (params (bWonGame :type Boolean))
  (bind _returnvalue (`|CreateWidget` "/Game/Blueprints/Widgets/WBP_EndGameWidget.WBP_EndGameWidget_C"))
  (`UserWidget.AddToViewport` _returnvalue 0)
  (`TextBlock.SetText` (`/Game/Blueprints/Widgets/WBP_EndGameWidget.DisplayText` _returnvalue) (select `bool` bWonGame :`false` "You Lose!" :`true` "You Win!" :!type "Text"))
  (set `PlayerController.bShowMouseCursor` true (`GameplayStatics.GetPlayerController` 0))
  (`GameplayStatics.SetGamePaused` true))

(fn `UserConstructionScript`)